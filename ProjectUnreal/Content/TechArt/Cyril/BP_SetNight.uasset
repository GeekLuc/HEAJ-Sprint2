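; BP_SetNight is an actor that switches the scene lighting to night once BPBille's CabaneOut flag is set.
; Each Tick it polls that flag and, while true, rotates the directional light along the NightLightRotation vector and sets the point light to its night intensity.
; The change is applied instantly and reapplied every frame, with no blend or return to day lighting.
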(event EventBeginPlay)

(event Collision|EventActorBeginOverlap
  (params (OtherActor :type Actor%20Object%20Reference)))

(event EventTick
  (params (DeltaSeconds :type Float%20%28single-precision%29))
  (if (Variables|/Game/Blueprints/Gameplay/Pawn/BP_GAMEPLAY_Bille.BP_GAMEPLAY_Bille_C|GetCabane_Out? (Variables|Default|GetBP_Bille))
    (Transformation|SetActorRotation (Variables|Default|GetDirectionalLight) (Math|Conversions|RotationFromXVector (Variables|Default|GetNightLightRotation)))
    (Rendering|Components|Light|SetIntensity (Variables|/Script/Engine.PointLight|GetPointLightComponent (Variables|Default|GetPointLight)) (Variables|Default|GetPointLightNightIntencity))))

(fn ConstructionScript)