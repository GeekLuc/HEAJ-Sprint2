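; Marble ("Bille") pawn that rolls itself along a target spline from its far end to the start, then triggers the gamemode's Win.
; After timed delays, Tick moves it at a DataTable-driven base speed, scaled for climbing or descending by comparing its height to the next spline point.
; It also tracks velocity and aligns the camera arm and board ("Planche") to the spline.
; A box overlap restores the player pawn's jump.
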(event OnComponentBeginOverlap(Box)
  (params (OverlappedComponent :type Primitive%20Component%20Object%20Reference) (OtherActor :type Actor%20Object%20Reference) (OtherComp :type Primitive%20Component%20Object%20Reference) (OtherBodyIndex :type Integer) (bFromSweep :type Boolean) (SweepResult :type Hit%20Result%20Structure%20%28by%20ref%29))
  (bind _asbp_gameplay_pawn_player (Utilities|Casting|CastToBP_GAMEPLAY_Pawn_Player OtherActor))
  (if (not (Variables|/Game/Blueprints/Gameplay/Pawn/BP_GAMEPLAY_Pawn_Player.BP_GAMEPLAY_Pawn_Player_C|GetCanJump? _asbp_gameplay_pawn_player))
    (Default|JumpEnd _asbp_gameplay_pawn_player)
    (Variables|/Game/Blueprints/Gameplay/Pawn/BP_GAMEPLAY_Pawn_Player.BP_GAMEPLAY_Pawn_Player_C|SetCanJump? _asbp_gameplay_pawn_player true)))

(event EventTick
  (params (DeltaSeconds :type Float%20%28single-precision%29))
  (if (Variables|Default|GetStart?)
    (if (not (Variables|Parameter|GetAtEndSpline))
      (CallFunction|MoveBille DeltaSeconds)
      (CallFunction|SetCamera)
      (CallFunction|SetRotatePlanche)
      (Variables|Parameter|SetBillyVelocity (/ (- (Transformation|GetActorLocation) (Variables|Parameter|GetPreviousPosition)) (Utilities|Time|GetWorldDeltaSeconds)))
      (Variables|Parameter|SetPreviousPosition (Transformation|GetActorLocation))
      (else
        (Variables|Parameter|SetBillyVelocity "0, 0, 0")
        (Utilities|FlowControl|Delay 0.5)
        (Default|Win (Variables|Ref|GetAs%20BP%20GAMEPLAY%20Gamemode))))))

(event EventBeginPlay
  (Variables|Parameter|SetDistance 0.0)
  (bind _asbp_gameplay_camera (Utilities|Casting|CastToBP_GAMEPLAY_Camera (Variables|/Script/Engine.ChildActorComponent|GetChildActor (Variables|Default|GetCamera))))
  (Variables|Ref|SetAs%20BP%20GAMEPLAY%20Camera _asbp_gameplay_camera)
  (bind _returnvalue (Utilities|GetDataTableRow "/Game/Blueprints/DataTable/DT_Player.DT_Player" "VitesseBaseBille")
    (:then
      (Variables|Parameter|SetSpeedBase (.value _returnvalue))
      (bind _returnvalue_2 (Utilities|GetDataTableRow "/Game/Blueprints/DataTable/DT_Player.DT_Player" "MultiplicateurMonter")
        (:then
          (Variables|Parameter|SetMultipl_monter (.value _returnvalue_2))
          (bind _returnvalue_3 (Utilities|GetDataTableRow "/Game/Blueprints/DataTable/DT_Player.DT_Player" "MultiplicateurDescendre")
            (:then
              (Variables|Parameter|SetMultipl_descendre (.value _returnvalue_3))
              (bind _asbp_gameplay_gamemode (Utilities|Casting|CastToBP_GAMEPLAY_Gamemode (Game|GetGameMode)))
              (Variables|Ref|SetAs%20BP%20GAMEPLAY%20Gamemode _asbp_gameplay_gamemode)
              (Utilities|FlowControl|Delay 1e+01)
              (Variables|Default|SetStartMove true)
              (bind _returnvalue_4 (Utilities|GetDataTableRow "/Game/Blueprints/DataTable/DT_Player.DT_Player" "Decompte")
                (:then
                  (Utilities|FlowControl|Delay (.value _returnvalue_4))
                  (Variables|Default|SetStart? true)
                  (Audio|PlaySound2D "/Game/Sounds/SC_Bille.SC_Bille" 1.0 1.0 0.0 0 0))))))))))

(fn ConstructionScript)

(fn MoveBille
  (params (Delta%20seconds :type Float%20%28double-precision%29))
  (bind _returnvalue (Transformation|GetActorLocation))
  (Variables|Parameter|SetDistance (- (Variables|Parameter|GetDistance) (* (* Delta%20seconds (Variables|Parameter|GetSpeed)) 1e+02)))
  (Variables|Parameter|SetDistanceInverse (+ (Spline|GetSplineLength (Variables|/Game/Blueprints/Gameplay/Pawn/BP_GAMEPLAY_SplinePath.BP_GAMEPLAY_SplinePath_C|GetSplinePath (Variables|Ref|GetTargetSpline))) (Variables|Parameter|GetDistance)))
  (if (> (.z _returnvalue) (.z (Spline|GetLocationatDistanceAlongSpline (Variables|/Game/Blueprints/Gameplay/Pawn/BP_GAMEPLAY_SplinePath.BP_GAMEPLAY_SplinePath_C|GetSplinePath (Variables|Ref|GetTargetSpline)) (Variables|Parameter|GetDistanceInverse) "World")))
    (Variables|Parameter|SetSpeed (Math|Float|Lerp (Variables|Parameter|GetSpeed) (* (Variables|Parameter|GetSpeedBase) (Variables|Parameter|GetMultipl_descendre)) 1.0))
    (elif (< (.z _returnvalue) (.z (Spline|GetLocationatDistanceAlongSpline (Variables|/Game/Blueprints/Gameplay/Pawn/BP_GAMEPLAY_SplinePath.BP_GAMEPLAY_SplinePath_C|GetSplinePath (Variables|Ref|GetTargetSpline)) (Variables|Parameter|GetDistanceInverse) "World")))
      (Variables|Parameter|SetSpeed (Math|Float|Lerp (Variables|Parameter|GetSpeed) (* (Variables|Parameter|GetSpeedBase) (Variables|Parameter|GetMultipl_monter)) 1.0))
      (else
        (Variables|Parameter|SetSpeed (Math|Float|Lerp (Variables|Parameter|GetSpeed) (Variables|Parameter|GetSpeedBase) 1.0)))))
  (Transformation|SetActorLocation (Math|Vector|MakeVector (.x (Spline|GetLocationatDistanceAlongSpline (Variables|/Game/Blueprints/Gameplay/Pawn/BP_GAMEPLAY_SplinePath.BP_GAMEPLAY_SplinePath_C|GetSplinePath (Variables|Ref|GetTargetSpline)) (Variables|Parameter|GetDistanceInverse) "World")) (.y (Spline|GetLocationatDistanceAlongSpline (Variables|/Game/Blueprints/Gameplay/Pawn/BP_GAMEPLAY_SplinePath.BP_GAMEPLAY_SplinePath_C|GetSplinePath (Variables|Ref|GetTargetSpline)) (Variables|Parameter|GetDistanceInverse) "World")) (.z (Spline|GetLocationatDistanceAlongSpline (Variables|/Game/Blueprints/Gameplay/Pawn/BP_GAMEPLAY_SplinePath.BP_GAMEPLAY_SplinePath_C|GetSplinePath (Variables|Ref|GetTargetSpline)) (Variables|Parameter|GetDistanceInverse) "World"))) false false)
  (if (<= (Variables|Parameter|GetDistanceInverse) 0.0)
    (Variables|Parameter|SetAtEndSpline true)
    (else
      (Variables|Parameter|SetAtEndSpline false))))

(fn SetCamera
  (bind _targetspline (Variables|Ref|GetTargetSpline))
  (bind _distanceinverse (Variables|Parameter|GetDistanceInverse))
  (bind _splinepath (Variables|/Game/Blueprints/Gameplay/Pawn/BP_GAMEPLAY_SplinePath.BP_GAMEPLAY_SplinePath_C|GetSplinePath _targetspline))
  (bind _returnvalue (Spline|GetRotationatDistanceAlongSpline _splinepath _distanceinverse "World"))
  (Transformation|SetWorldRotation (Variables|/Game/Blueprints/Gameplay/Pawn/BP_GAMEPLAY_Camera.BP_GAMEPLAY_Camera_C|GetSpringArm (Variables|Ref|GetAs%20BP%20GAMEPLAY%20Camera)) (Math|Rotator|MakeRotator (.roll _returnvalue) (.pitch (Transformation|GetWorldRotation (Variables|Default|GetCamera))) (+ (.yaw _returnvalue) 1.8e+02)) false false))

(fn SetRotatePlanche
  (bind _targetspline (Variables|Ref|GetTargetSpline))
  (bind _distanceinverse (Variables|Parameter|GetDistanceInverse))
  (bind _splinepath (Variables|/Game/Blueprints/Gameplay/Pawn/BP_GAMEPLAY_SplinePath.BP_GAMEPLAY_SplinePath_C|GetSplinePath _targetspline))
  (bind _returnvalue (Spline|GetRotationatDistanceAlongSpline _splinepath _distanceinverse "World"))
  (Transformation|SetWorldRotation (Variables|Default|GetPlanche) (Math|Rotator|MakeRotator (.roll _returnvalue) (Math|Float|Clamp(Float) (.pitch _returnvalue) -3e+01 3e+01) (.yaw _returnvalue)) false false))