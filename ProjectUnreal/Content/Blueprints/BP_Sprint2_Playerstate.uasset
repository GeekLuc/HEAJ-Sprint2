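; Player state for local multiplayer that holds each player's name and visual identity: skeletal, anim blueprint, icon material and player material.
; SetVariables derives the name and DT_Player row (Joueur1 to Joueur4) from the current player controller count, printing debug errors when the row is missing.
; GetPlayerInfos exposes the cached values, and destruction of the state also destroys its FakePlayer actor if valid.
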(event Custom|SetVariables
  (bind _returnvalue (Class|GameplayStatics|GetNumPlayerControllers))
  (bind _returnvalue_2 (- _returnvalue 1))
  (bind _returnvalue_3 (Utilities|Select :Index _returnvalue_2 :Option%200 "Joueur1" :Option%201 "Joueur2" :Option%202 "Joueur3" :Option%203 "Joueur4"))
  (Variables|Default|SetName (Utilities|String|Append "Player " (Utilities|String|ToString(Integer) (Class|GameplayStatics|GetNumPlayerControllers))))
  (bind _returnvalue_4 (Utilities|GetDataTableRow "/Game/Blueprints/DataTable/DT_Player.DT_Player" _returnvalue_3)
    (:then
      (Variables|Default|SetSkeletal (.skeletal _returnvalue_4))
      (Variables|Default|SetABP (.abp _returnvalue_4))
      (Variables|Default|SetMat_Icone (.mat_icone _returnvalue_4))
      (Variables|Default|SetMat_Player (.mat_players _returnvalue_4)))
    (:RowNotFound
      (Development|PrintString "LIGNE DE LA DATA PAS TROUVER" true true "(R=1.000000,G=0.021504,B=0.000000,A=1.000000)" 15.0)
      (Development|PrintString (Utilities|String|ToString(Name) _returnvalue_3) true true "(R=1.000000,G=0.021504,B=0.000000,A=1.000000)" 15.0))))

(event EventDestroyed
  (bind _fakeplayer (Variables|Default|GetFakePlayer)
    (:then
      (Actor|DestroyActor _fakeplayer))
    (:else)))

(fn ConstructionScript)

(fn GetPlayerInfos
  (return (Variables|Default|GetName) (Variables|Default|GetSkeletal) (Variables|Default|GetABP) (Variables|Default|GetMat_Icone) (Variables|Default|GetMat_Player)))